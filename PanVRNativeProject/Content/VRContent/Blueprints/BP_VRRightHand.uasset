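; BP_VRRightHand is the right-hand VR hand Blueprint, animating a demon hand mesh and handling grabbing.
; Enhanced Input grasp and index-curl actions write their values to pose alphas on the ABP_DemonHand anim instance, resetting them to zero on cancel or completion.
; The right grab action calls GrabObject when started and ReleaseObject when canceled or completed.
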(event `self.ReceiveBeginPlay`
  (`parent.ReceiveBeginPlay`))

(event `EnhancedInput|/Game/VRTemplate/Input/Actions/Hands/IA_Hand_Grasp_Right`
  (params (ActionValue :type "Float (double-precision)") (ElapsedSeconds :type "Float (double-precision)") (TriggeredSeconds :type "Float (double-precision)") (InputAction :type "InputAction Object Reference" :default "/Game/VRTemplate/Input/Actions/Hands/IA_Hand_Grasp_Right.IA_Hand_Grasp_Right"))
  (bind _returnvalue (`SkeletalMeshComponent.GetAnimInstance` (`self.HandMesh`)))
  (:`Triggered`
    (bind _asabp_demon_hand (cast `/Game/VRContent/HandRelated/HandAnimation/ABP_DemonHand` _returnvalue))
    (set `/Game/VRContent/HandRelated/HandAnimation/ABP_DemonHand.PoseAlphaGrasp` ActionValue _asabp_demon_hand))
  (:`Canceled`
    (bind _asabp_demon_hand_2 (cast `/Game/VRContent/HandRelated/HandAnimation/ABP_DemonHand` _returnvalue :!label _label))
    (set `/Game/VRContent/HandRelated/HandAnimation/ABP_DemonHand.PoseAlphaGrasp` 0.0 _asabp_demon_hand_2))
  (:`Completed`
    (goto _label)))

(event `EnhancedInput|/Game/VRTemplate/Input/Actions/Hands/IA_Hand_IndexCurl_Right`
  (params (ActionValue :type "Float (double-precision)") (ElapsedSeconds :type "Float (double-precision)") (TriggeredSeconds :type "Float (double-precision)") (InputAction :type "InputAction Object Reference" :default "/Game/VRTemplate/Input/Actions/Hands/IA_Hand_IndexCurl_Right.IA_Hand_IndexCurl_Right"))
  (bind _returnvalue (`SkeletalMeshComponent.GetAnimInstance` (`self.HandMesh`)))
  (:`Triggered`
    (bind _asabp_demon_hand (cast `/Game/VRContent/HandRelated/HandAnimation/ABP_DemonHand` _returnvalue))
    (set `/Game/VRContent/HandRelated/HandAnimation/ABP_DemonHand.PoseAlphaIndexCurl` ActionValue _asabp_demon_hand))
  (:`Canceled`
    (bind _asabp_demon_hand_2 (cast `/Game/VRContent/HandRelated/HandAnimation/ABP_DemonHand` _returnvalue :!label _label_2))
    (set `/Game/VRContent/HandRelated/HandAnimation/ABP_DemonHand.PoseAlphaIndexCurl` 0.0 _asabp_demon_hand_2))
  (:`Completed`
    (goto _label_2)))

(event `EnhancedInput|/Game/VRTemplate/Input/Actions/IA_Grab_Right`
  (params (ActionValue :type "Float (double-precision)") (ElapsedSeconds :type "Float (double-precision)") (TriggeredSeconds :type "Float (double-precision)") (InputAction :type "InputAction Object Reference" :default "/Game/VRTemplate/Input/Actions/IA_Grab_Right.IA_Grab_Right"))
  (:`Started`
    (`self.GrabObject`))
  (:`Canceled`
    (`self.ReleaseObject` :!label _label_3))
  (:`Completed`
    (goto _label_3)))

(fn `UserConstructionScript`
  (`parent.UserConstructionScript`))